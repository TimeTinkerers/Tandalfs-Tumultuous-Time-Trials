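; BP_BoulderTrigger is a one-shot box trigger that clears a boulder and rubble behind a blacked-out, audio-only cutscene.
; When BP_ThirdPersonCharacter overlaps the box, it disables input and fades the camera to black.
; While the screen stays dark, it plays the cutscene sound and hides the referenced boulder and rubble with collision off.
; After timed delays it fades back in, restores input and destroys itself.
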(event `self.Box.OnComponentBeginOverlap`
  (params (OverlappedComponent :type "PrimitiveComponent Object Reference") (OtherActor :type "Actor Object Reference") (OtherComp :type "PrimitiveComponent Object Reference") (OtherBodyIndex :type Integer) (bFromSweep :type Boolean) (SweepResult :type "HitResult Structure (by ref)"))
  (cast `/Game/ThirdPerson/Blueprints/BP_ThirdPersonCharacter` OtherActor)
  (`self.DisableInput` (`GameplayStatics.GetPlayerController` 0))
  (`PlayerCameraManager.StartCameraFade` (`GameplayStatics.GetPlayerCameraManager` 0) 0.0 1.0 1.5 (struct :`A` 1.0) false true)
  (`KismetSystemLibrary.Delay` 1.5)
  (`GameplayStatics.PlaySoundAtLocation` "/Game/Audio/cutscene_sound.cutscene_sound" (`self.K2_GetActorLocation`) (struct) 1.0 1.0 0.0 null null null null)
  (`self.SetActorHiddenInGame` (`self.OutRubble`) true)
  (`self.SetActorEnableCollision` (`self.OutRubble`) false)
  (`self.SetActorHiddenInGame` (`self.BoulderRef`) true)
  (`self.SetActorEnableCollision` (`self.BoulderRef`) false)
  (`KismetSystemLibrary.Delay` 6.0)
  (`PlayerCameraManager.StartCameraFade` :`self` (`GameplayStatics.GetPlayerCameraManager` 0) :`FromAlpha` 1.0 :`Duration` 1.5)
  (`self.EnableInput` (`GameplayStatics.GetPlayerController` 0))
  (`self.K2_DestroyActor`))

(fn `UserConstructionScript`)