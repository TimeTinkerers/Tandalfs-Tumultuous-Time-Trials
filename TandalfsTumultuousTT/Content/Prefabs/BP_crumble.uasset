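; BP_crumble is a moving platform that oscillates continuously from its starting location and can be temporarily frozen.
; On BeginPlay it caches its location, then a Timeline adds a movement offset to it.
; Finished alternates the Timeline between forward and reverse play for an endless loop.
; PlatformFreeze suppresses location updates for a few seconds while the Timeline keeps running, so the platform snaps to the current offset afterwards.
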(event `self.ReceiveBeginPlay`
  (set `self.PlatformMove` (`self.K2_GetActorLocation`))
  (`self.PlatformEnd`))

(event `PlatformEnd`
  (bind (_direction _move) (`Timeline|Timeline` :!via `PlayFromStart` :!label _label)
    (:`Update`
      (if (not (`self.isFrozen`))
        (`self.K2_SetActorLocation` (+ (`self.PlatformMove`) _move))))
    (:`Finished`
      (switch `ETimelineDirection` _direction
        (:`Forward`
          (`self.PlatformStart`))
        (:`Backward`
          (`self.PlatformEnd`))))))

(event `PlatformStart`
  (goto _label :!via `ReverseFromEnd`))

(event `PlatformFreeze`
  (set `self.isFrozen` true)
  (`KismetSystemLibrary.Delay` 3.0)
  (set `self.isFrozen` false))

(fn `UserConstructionScript`)